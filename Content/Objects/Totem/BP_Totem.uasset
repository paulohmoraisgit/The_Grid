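; Interactable totem for one of three color types (pink, green, blue) that spawns a key and can activate itself.
; The first Interact attempts activation, then spawns a BP_KeyFixo tinted to the totem's color through dynamic glow materials.
; Activation requires the matching key-picked flag in BP_GameplayGameMode, then plays the ring timeline, raises the base's emissive and updates the game mode's active-totem count and all-active check.
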(event Custom|ActiveTotemPink
  (bind _gamemoderefer (Variables|Default|GetGameModeRefer))
  ;[1 1 1] Eventos de Ativação dos Totem - Checa isPickKey - Toca a Animação do Aro
  (if (Variables|/Game/GameLogic/BP_GameplayGameMode.BP_GameplayGameMode_C|GetisPickKeyPink (Variables|Default|GetGameModeRefer))
    (Components|Timeline|PlayfromStart (Variables|Default|GetAroTimeline))
    (Rendering|Material|SetScalarParameterValue (Variables|Default|GetTotemMaterial) "Emissive" (Variables|Default|GetEmissiveIntensityActive) :!class /Script/Engine.MaterialInstanceDynamic)
    (Default|IncrementNumberTotemsActive _gamemoderefer)
    (Default|CheckAllTotemsActive _gamemoderefer)))

(event Custom|ActiveTotemGreen
  (bind _gamemoderefer (Variables|Default|GetGameModeRefer))
  ;[1 1 1] Eventos de Ativação dos Totem - Checa isPickKey - Toca a Animação do Aro
  (if (Variables|/Game/GameLogic/BP_GameplayGameMode.BP_GameplayGameMode_C|GetisPickKeyGreen (Variables|Default|GetGameModeRefer))
    (Components|Timeline|PlayfromStart (Variables|Default|GetAroTimeline))
    (Rendering|Material|SetScalarParameterValue (Variables|Default|GetTotemMaterial) "Emissive" (Variables|Default|GetEmissiveIntensityActive) :!class /Script/Engine.MaterialInstanceDynamic)
    (Default|IncrementNumberTotemsActive _gamemoderefer)
    (Default|CheckAllTotemsActive _gamemoderefer)))

(event Custom|ActiveTotemBlue
  (bind _gamemoderefer (Variables|Default|GetGameModeRefer))
  ;[1 1 1] Eventos de Ativação dos Totem - Checa isPickKey - Toca a Animação do Aro
  (if (Variables|/Game/GameLogic/BP_GameplayGameMode.BP_GameplayGameMode_C|GetisPickKeyBlue (Variables|Default|GetGameModeRefer))
    (Components|Timeline|PlayfromStart (Variables|Default|GetAroTimeline))
    (Rendering|Material|SetScalarParameterValue (Variables|Default|GetTotemMaterial) "Emissive" (Variables|Default|GetEmissiveIntensityActive) :!class /Script/Engine.MaterialInstanceDynamic)
    (Default|IncrementNumberTotemsActive _gamemoderefer)
    (Default|CheckAllTotemsActive _gamemoderefer)))

(event EventBeginPlay
  ;[1 1 1] Begin Play - Get Game Mode Reference
  (bind _asbp_gameplay_game_mode (Utilities|Casting|CastToBP_GameplayGameMode (Game|GetGameMode)))
  (Variables|Default|SetGameModeRefer _asbp_gameplay_game_mode))

(event EventInteract
  (bind _totemscolor (Variables|Default|GetTotemsColor))
  (bind (_blue _green) (Utilities|Struct|BreakColorsStruct _totemscolor))
  ;[1 1 1] Blueprint Interface - Lógica de Interação que ativa o Totem - Spawn Actor de Classe Key - Cria Material de cor específica para a Chave
  (switch Utilities|FlowControl|Switch|SwitchonEKeys (Variables|Default|GetTotemType)
    (:NewEnumerator0
      (Utilities|FlowControl|DoOnce false
        (:Completed
          (CallFunction|ActiveTotemPink)
          (bind _returnvalue (CallFunction|SpawnKey))
          (CallFunction|CreateKeyMaterial (Variables|/Game/Objects/Key/BP_KeyFixo.BP_KeyFixo_C|GetFrame1 _returnvalue) (Variables|/Game/Objects/Key/BP_KeyFixo.BP_KeyFixo_C|GetFrame2 _returnvalue) (.Pink (Utilities|Struct|BreakColorsStruct (Variables|Default|GetTotemsColor)))))))
    (:NewEnumerator1
      (Utilities|FlowControl|DoOnce false
        (:Completed
          (CallFunction|ActiveTotemGreen)
          (bind _returnvalue_2 (CallFunction|SpawnKey))
          (CallFunction|CreateKeyMaterial (Variables|/Game/Objects/Key/BP_KeyFixo.BP_KeyFixo_C|GetFrame1 _returnvalue_2) (Variables|/Game/Objects/Key/BP_KeyFixo.BP_KeyFixo_C|GetFrame2 _returnvalue_2) _green))))
    (:NewEnumerator2
      (Utilities|FlowControl|DoOnce false
        (:Completed
          (CallFunction|ActiveTotemBlue)
          (bind _returnvalue_3 (CallFunction|SpawnKey))
          (CallFunction|CreateKeyMaterial (Variables|/Game/Objects/Key/BP_KeyFixo.BP_KeyFixo_C|GetFrame1 _returnvalue_3) (Variables|/Game/Objects/Key/BP_KeyFixo.BP_KeyFixo_C|GetFrame2 _returnvalue_3) _blue))))))

(fn ConstructionScript
  (bind _returnvalue (Rendering|Material|CreateDynamicMaterialInstance (Variables|Default|GetTotemBase) 1 "/Game/Materiais/M_Glow.M_Glow" :!class /Script/Engine.PrimitiveComponent))
  (bind _output_get (Variables|Default|SetTotemMaterial _returnvalue))
  (Rendering|Material|SetScalarParameterValue _output_get "Emissive" (Variables|Default|GetEmissiveIntensity) :!class /Script/Engine.MaterialInstanceDynamic)
  (Rendering|Material|SetVectorParameterValue _output_get "BaseColor" (Variables|Default|GetBaseColor) :!class /Script/Engine.MaterialInstanceDynamic))

(fn SpawnKey
  (bind _returnvalue (Game|SpawnActorfromClass "/Game/Objects/Key/BP_KeyFixo.BP_KeyFixo_C" (Transformation|GetWorldTransform (Variables|Default|GetKeySpawnTransform)) "Undefined" 0 0))
  (return _returnvalue))

(fn CreateKeyMaterial
  (params (Target :type Primitive%20Component%20Object%20Reference) (Target2 :type Primitive%20Component%20Object%20Reference) (Cor :type Linear%20Color%20Structure))
  (bind _returnvalue (Rendering|Material|CreateDynamicMaterialInstance Target 1 "/Game/Materiais/M_Glow.M_Glow" :!class /Script/Engine.PrimitiveComponent))
  (Rendering|Material|SetVectorParameterValue _returnvalue "BaseColor" Cor :!class /Script/Engine.MaterialInstanceDynamic)
  (Rendering|Material|SetScalarParameterValue _returnvalue "Emissive" 2e+01 :!class /Script/Engine.MaterialInstanceDynamic)
  (bind _returnvalue_2 (Rendering|Material|CreateDynamicMaterialInstance Target2 1 "/Game/Materiais/M_Glow.M_Glow" :!class /Script/Engine.PrimitiveComponent))
  (Rendering|Material|SetVectorParameterValue _returnvalue_2 "BaseColor" Cor :!class /Script/Engine.MaterialInstanceDynamic)
  (Rendering|Material|SetScalarParameterValue _returnvalue_2 "Emissive" 2e+01 :!class /Script/Engine.MaterialInstanceDynamic))