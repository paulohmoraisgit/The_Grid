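; BP_Portal2 is a portal that teleports the player hero when anything overlaps its mesh, as the overlapping actor is never checked.
; A looping timer replays a timeline that moves the mesh from start to end location, then snaps it back.
; On overlap it searches all BP_DestinationBillboard2 actors for a match to DestinationPoint, stops the hero's movement and applies that actor's location and control rotation.
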(event OnComponentBeginOverlap(PortalMesh)
  (params (OverlappedComponent :type Primitive%20Component%20Object%20Reference) (OtherActor :type Actor%20Object%20Reference) (OtherComp :type Primitive%20Component%20Object%20Reference) (OtherBodyIndex :type Integer) (bFromSweep :type Boolean) (SweepResult :type Hit%20Result%20Structure%20%28by%20ref%29))
  (bind _hero_refer (Variables|Default|GetHero%20Refer))
  (bind _outactors (Actor|GetAllActorsOfClass "/Game/Objects/Portal/BP_DestinationBillboard2.BP_DestinationBillboard2_C"))
  (for _array_element _outactors
    (if (== (Variables|/Game/Objects/Portal/BP_DestinationBillboard2.BP_DestinationBillboard2_C|GetDestinationBillboard _array_element) (Variables|Default|GetdestinationPoint))
      (Components|Movement|StopMovementImmediately (Variables|/Script/Engine.Character|GetCharacterMovement (Variables|Default|GetHero%20Refer)))
      (Transformation|SetActorLocation _hero_refer (Transformation|GetActorLocation _array_element) false false)
      (Pawn|SetControlRotation (Pawn|GetController _hero_refer) (Transformation|GetActorRotation _array_element)))))

(event Custom|PlayPortal
  ;[1 1 1] PortalMesh: Create Timer to Timeline, Play Timeline Location
  (bind _portalmove (Timeline|PortalAnimation PlayFromStart)
    (:Update
      (Transformation|SetRelativeLocation (Variables|Default|GetPortalMesh) (Math|Vector|Lerp(Vector) (Variables|Default|GetStartLocation) (Variables|Default|GetEndLocation) _portalmove) false false))
    (:Finished
      (Transformation|SetRelativeLocation (Variables|Default|GetPortalMesh) (Variables|Default|GetStartLocation) false false))))

(event EventBeginPlay
  ;[1 1 1] Create Hero Refer
  (bind _asbp_hero_char (Utilities|Casting|CastToBP_HeroChar (Game|GetPlayerCharacter 0)))
  (Variables|Default|SetHero%20Refer _asbp_hero_char)
  ;[1 1 1] PortalMesh: Create Timer to Timeline, Play Timeline Location
  (Utilities|Time|SetTimerbyEvent (delegate Custom|PlayPortal) (Variables|Default|GetPortalTime) true))

(fn ConstructionScript)