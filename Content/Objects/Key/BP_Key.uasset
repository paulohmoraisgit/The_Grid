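; BP_Key is a key object whose Pickup function returns its KeyColor to the caller.
; Two timelines define its animation: one yaws Frame1 and bobs Core vertically, the other pitches Frame2.
; No event in the graph starts either timeline, so the animation depends on autoplay or an external trigger.
; Pickup only returns the color, and the construction script is empty.
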(fn ConstructionScript)

(fn Pickup
  (return (Variables|Default|GetKeyColor)))