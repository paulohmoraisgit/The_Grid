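; BP_KeyPink is the pink variant of a key object, setting its glowing color.
; Its Construction Script calls the parent, then creates dynamic M_Glow instances on material slot 1 of Frame1 and Frame2.
; Both instances take the pink entry from KeysColor as base color and a strong emissive value.
; The Event Graph holds only disabled default events, so the file adds no gameplay logic.
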(event EventBeginPlay
  (|CallParentFunction) ; This node is disabled and will not be called.\nDrag off pins to build functionality.
)

(event Collision|EventActorBeginOverlap
  (params (OtherActor :type Actor%20Object%20Reference))
  (|CallParentFunction OtherActor) ; This node is disabled and will not be called.\nDrag off pins to build functionality.
)

(event EventTick
  (params (DeltaSeconds :type Float%20%28single-precision%29))
  (|CallParentFunction DeltaSeconds) ; This node is disabled and will not be called.\nDrag off pins to build functionality.
)

(fn ConstructionScript
  (bind _keyscolor (Variables|Default|GetKeysColor))
  (bind _pink (Utilities|Struct|BreakColorsStruct _keyscolor))
  (|CallParentFunction)
  (bind _returnvalue (Rendering|Material|CreateDynamicMaterialInstance (Variables|Default|GetFrame1) 1 "/Game/Materiais/M_Glow.M_Glow" :!class /Script/Engine.PrimitiveComponent))
  (Rendering|Material|SetVectorParameterValue _returnvalue "BaseColor" _pink :!class /Script/Engine.MaterialInstanceDynamic)
  (Rendering|Material|SetScalarParameterValue _returnvalue "Emissive" 2e+01 :!class /Script/Engine.MaterialInstanceDynamic)
  (bind _returnvalue_2 (Rendering|Material|CreateDynamicMaterialInstance (Variables|Default|GetFrame2) 1 "/Game/Materiais/M_Glow.M_Glow" :!class /Script/Engine.PrimitiveComponent))
  (Rendering|Material|SetVectorParameterValue _returnvalue_2 "BaseColor" _pink :!class /Script/Engine.MaterialInstanceDynamic)
  (Rendering|Material|SetScalarParameterValue _returnvalue_2 "Emissive" 2e+01 :!class /Script/Engine.MaterialInstanceDynamic))