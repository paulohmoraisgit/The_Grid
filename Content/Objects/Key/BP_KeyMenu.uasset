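; BP_KeyMenu is a menu variant of the key object that reacts to player input and opens the gameplay level when the pause button is pressed.
; Two timelines, with no wired play input, drive the rotation of two frames and the core's vertical bob.
; MoveForward scales the timelines' play rate, while MoveRight drives the frames' clamped emissive glow.
; A Pickup function returns the key's color.
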(event Input|ActionEvents|InputActionPauseButton
  (params (Key :type Key%20Structure))
  (:Pressed
    (Game|OpenLevel(byName) "01Gameplay")))

(event Input|AxisEvents|InputAxisMoveForward
  (params (AxisValue :type Float%20%28single-precision%29))
  (bind _returnvalue (* AxisValue 2.0))
  (bind _returnvalue_2 (+ _returnvalue 0.5))
  (Components|Timeline|SetPlayRate (Variables|Default|GetTimeline_1) _returnvalue_2)
  (Components|Timeline|SetPlayRate (Variables|Default|GetTimeline_0) _returnvalue_2))

(event Input|AxisEvents|InputAxisMoveRight
  (params (AxisValue :type Float%20%28single-precision%29))
  (bind _returnvalue (Math|Float|Clamp(Float) AxisValue 0.2))
  (bind _returnvalue_2 (* _returnvalue 8e+01))
  (Rendering|Material|SetScalarParameterValueonMaterials (Variables|Default|GetFrame1) "Emissive" _returnvalue_2)
  (Rendering|Material|SetScalarParameterValueonMaterials (Variables|Default|GetFrame2) "Emissive" _returnvalue_2))

(fn ConstructionScript)

(fn Pickup
  (return (Variables|Default|GetKeyColor)))