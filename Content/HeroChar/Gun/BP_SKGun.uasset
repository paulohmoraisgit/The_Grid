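; BP_SKGun is the hero's automatic gun, firing BP_Projetil projectiles while its trigger is active.
; On BeginPlay it caches the player's BP_HeroChar, whose ArrowProjetil component supplies each shot's spawn transform.
; ActiveTrigger fires immediately, then repeats FireAndPlaySound on a looping timer set by ShootPerSecond, until DeactiveTrigger clears it.
; Each shot spawns a projectile and plays the fire sound at the arrow's location.
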(event Custom|ActiveTrigger
  ;[1 1 1] Active Trigger / Deactive Trigger / Fire
  (CallFunction|FireandPlaySound)
  (Utilities|Time|SetTimerbyFunctionName 0 "FireAndPlaySound" (/ 1.0 (Variables|Default|GetShootPerSecond)) true))

(event Custom|DeactiveTrigger
  ;[1 1 1] Active Trigger / Deactive Trigger / Fire
  (Utilities|Time|ClearTimerbyFunctionName 0 "FireAndPlaySound"))

(event EventBeginPlay
  ;[1 1 1] Get HeroChar Refer
  (bind _asbp_hero_char (Utilities|Casting|CastToBP_HeroChar (Game|GetPlayerCharacter 0)))
  (Variables|Default|SetHeroRefer _asbp_hero_char))

(fn ConstructionScript)

(fn FireandPlaySound
  (bind _herorefer (Variables|Default|GetHeroRefer))
  (bind _arrowprojetil (Variables|/Game/HeroChar/BP_HeroChar.BP_HeroChar_C|GetArrowProjetil _herorefer))
  (bind _returnvalue (Transformation|GetWorldTransform _arrowprojetil))
  (Game|SpawnActorfromClass "/Game/HeroChar/Gun/BP_Projetil.BP_Projetil_C" (Math|Transform|MakeTransform (.location _returnvalue) (.rotation _returnvalue) (.scale _returnvalue)) "Undefined" 0 0)
  ;[0.2292 0.1772 0.02148] Play Sound Fire
  (Audio|SpawnSoundatLocation "/Game/Audio/tiro4.tiro4" (.location _returnvalue)))