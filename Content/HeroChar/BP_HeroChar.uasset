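; First-person player character with walk, sprint, jump, look, pause and firing through a BP_SKGun attached to the arms.
; Interact sphere-traces from the camera, collecting colored keys via BI_Pickup or messaging BI_Interactble actors.
; Damage starts a DoOnce-guarded looping timer that restores health until full, with UI updates through the gameplay GameMode.
; Death runs once until reset, stopping fire and calling HeroDead.
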(event Custom|HeroDamage
  (params (Damage :type Float%20%28single-precision%29))
  ;[1 1 1] Hero Damage
  (Utilities|FlowControl|Sequence
    (:then_0
      (Variables|Default|SetCurrentHealth (- (Variables|Default|GetCurrentHealth) Damage))
      (if (<= (Variables|Default|GetCurrentHealth) 0.0)
        (Variables|Default|SetCurrentHealth 0.0)
        (CallFunction|Dead)
        (Default|UpdateUI (Variables|Default|GetGameplayGameModeRefer))
        (else
          (Default|UpdateUI (Variables|Default|GetGameplayGameModeRefer)))))
    (:then_1
      ;[1 1 1] Set Timer -  Chama Restaura Vida em Loop
      (Utilities|FlowControl|DoOnce false
        (:Completed
          (Utilities|Time|SetTimerbyFunctionName 0 "RestoreHealth" (Variables|Default|GetRestoreHealthTime) true))))))

(event Custom|HeroRestartDeadState
  ;[1 0.05729 0.05729] Morte
  (Utilities|FlowControl|DoOnce false) ; enters at Reset
)

(event Custom|RestoreHealth
  ;[1 1 1] Restaura Vida - Clear Timer quando a vida chega em 100
  (Variables|Default|SetCurrentHealth (+ (Variables|Default|GetCurrentHealth) (Variables|Default|GetRestoredHealth)))
  (if (>= (Variables|Default|GetCurrentHealth) (Variables|Default|GetTotalHealth))
    (Variables|Default|SetCurrentHealth (Variables|Default|GetTotalHealth))
    (Utilities|Time|ClearTimerbyFunctionName 0 "RestoreHealth")
    (CallFunction|ResetRestoreHealth)
    (Default|UpdateUI (Variables|Default|GetGameplayGameModeRefer))
    (else
      (Default|UpdateUI (Variables|Default|GetGameplayGameModeRefer)))))

(event Custom|ResetRestoreHealth
  ;[1 1 1] Set Timer -  Chama Restaura Vida em Loop
  (Utilities|FlowControl|DoOnce false) ; enters at Reset
)

(event Custom|Dead
  ;[1 0.05729 0.05729] Morte
  (Utilities|FlowControl|DoOnce false
    (:Completed
      (Variables|Default|SetisDead true)
      (Variables|Default|SetisFiring false)
      (Default|DeactiveTrigger (Variables|Default|GetBPGunRefer))
      (Default|CallHeroDead))))

(event EventBeginPlay
  (bind _arms (Variables|Default|GetArms))
  (Utilities|FlowControl|Sequence
    (:then_0
      ;[1 1 1] Set Max Walk Speed
      (Variables|/Script/Engine.CharacterMovementComponent|SetMaxWalkSpeed (Variables|Character|GetCharacterMovement) (Variables|Default|GetWalkSpeed)))
    (:then_1
      ;[1 1 1] Spawn BP Gun
      (bind _returnvalue (Game|SpawnActorfromClass "/Game/HeroChar/Gun/BP_SKGun.BP_SKGun_C" (Transformation|GetWorldTransform _arms) "Undefined" 0 0))
      (bind _output_get (Variables|Default|SetBPGunRefer _returnvalue))
      (Transformation|AttachComponentToComponent _output_get _arms "hand_rSocket" "SnapToTarget" "SnapToTarget" "SnapToTarget" true))
    (:then_2
      ;[1 1 1] Get GameMode Refer
      (bind _asbp_gameplay_game_mode (Utilities|Casting|CastToBP_GameplayGameMode (Game|GetGameMode)))
      (Variables|Default|SetGameplayGameModeRefer _asbp_gameplay_game_mode))))

(event Input|ActionEvents|InputActionJumpButton
  (params (Key :type Key%20Structure :default "None"))
  ;[1 1 1] Pulo
  (:Pressed
    (Character|Jump))
  (:Released
    (Character|StopJumping)))

(event Input|ActionEvents|InputActionSprintButton
  (params (Key :type Key%20Structure :default "None"))
  (bind _charactermovement (Variables|Character|GetCharacterMovement))
  ;[1 1 1] Corrida
  (:Pressed
    (Variables|Default|SetisSprinting true)
    (Variables|/Script/Engine.CharacterMovementComponent|SetMaxWalkSpeed _charactermovement (Variables|Default|GetSprintSpeed)))
  (:Released
    (Variables|Default|SetisSprinting false)
    (Variables|/Script/Engine.CharacterMovementComponent|SetMaxWalkSpeed _charactermovement (Variables|Default|GetWalkSpeed))))

(event Input|ActionEvents|InputActionFireButton
  (params (Key :type Key%20Structure :default "None"))
  ;[1 1 1] Tiro
  (:Pressed
    (Default|ActiveTrigger (Variables|Default|GetBPGunRefer))
    (Variables|Default|SetisFiring true))
  (:Released
    (Default|DeactiveTrigger (Variables|Default|GetBPGunRefer))
    (Variables|Default|SetisFiring false)))

(event Input|ActionEvents|InputActionPauseButton
  (params (Key :type Key%20Structure :default "None"))
  ;[1 1 1] Pause
  (:Pressed
    (if (Game|IsGamePaused)
      (Default|UnpauseGame (Variables|Default|GetGameplayGameModeRefer))
      (else
        (Default|PauseGame (Variables|Default|GetGameplayGameModeRefer))))))

(event Input|ActionEvents|InputActionInteractButton
  (params (Key :type Key%20Structure :default "None"))
  (bind _camera (Variables|Default|GetCamera))
  (bind _returnvalue (Transformation|GetWorldLocation _camera))
  ;[1 1 1] Interação com Sphere Trace - Confere se o Objeto que interage é Pickup ou Interactable
  (:Pressed
    (bind _outhit (Collision|SphereTraceByChannel _returnvalue (+ _returnvalue (* (Math|Vector|GetForwardVector _camera) 3e+02)) 1e+02 "TraceTypeQuery1" false 0 "None"))
    (if (Utilities|DoesObjectImplementInterface (.HitActor (Collision|BreakHitResult _outhit)) "/Game/Objects/Key/BI_Pickup.BI_Pickup_C")
      (bind _keycolor (Class|BIPickup|Pickup(Message) (.HitActor (Collision|BreakHitResult _outhit))))
      (switch Utilities|FlowControl|Switch|SwitchonEKeys _keycolor
        (:NewEnumerator0
          (Default|CallPickKeyPink)
          (Actor|DestroyActor (.HitActor (Collision|BreakHitResult _outhit))))
        (:NewEnumerator1
          (Default|CallPickKeyGreen)
          (Actor|DestroyActor (.HitActor (Collision|BreakHitResult _outhit))))
        (:NewEnumerator2
          (Default|CallPickKeyBlue)
          (Actor|DestroyActor (.HitActor (Collision|BreakHitResult _outhit)))))
      (elif (Utilities|DoesObjectImplementInterface (.HitActor (Collision|BreakHitResult _outhit)) "/Game/Objects/Totem/BI_Interactble.BI_Interactble_C")
        (Class|BIInteractble|Interact(Message) (.HitActor (Collision|BreakHitResult _outhit)))))))

(event Input|AxisEvents|InputAxisMoveForward
  (params (AxisValue :type Float%20%28single-precision%29))
  ;[1 1 1] Movimento Básico
  (Pawn|Input|AddMovementInput (Math|Vector|GetForwardVector (Variables|Collision|GetCapsuleComponent)) AxisValue false))

(event Input|AxisEvents|InputAxisMoveRight
  (params (AxisValue :type Float%20%28single-precision%29))
  ;[1 1 1] Movimento Básico
  (Pawn|Input|AddMovementInput (Math|Vector|GetRightVector (Variables|Collision|GetCapsuleComponent)) AxisValue false))

(event Input|AxisEvents|InputAxisLookTurn
  (params (AxisValue :type Float%20%28single-precision%29))
  ;[1 1 1] Movimento Básico
  (Pawn|Input|AddControllerYawInput AxisValue))

(event Input|AxisEvents|InputAxisLookUp
  (params (AxisValue :type Float%20%28single-precision%29))
  ;[1 1 1] Movimento Básico
  (Pawn|Input|AddControllerPitchInput AxisValue))

(fn ConstructionScript)