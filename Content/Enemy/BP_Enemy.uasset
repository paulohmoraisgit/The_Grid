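; BP_Enemy is a shooting enemy, with a boss variant, that turns toward the player once its capsule is overlapped or it gets hit.
; Alerting starts a looping Fire timer through a resettable DoOnce, spawning projectiles, doubled for bosses.
; Hits subtract health, briefly change emissive, and destroy the actor at zero, while separate events handle stopping and resetting.
; A randomized vertical bob timeline is set up, but nothing in the graph starts it.
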(event OnComponentBeginOverlap(Capsule)
  (params (OverlappedComponent :type Primitive%20Component%20Object%20Reference) (OtherActor :type Actor%20Object%20Reference) (OtherComp :type Primitive%20Component%20Object%20Reference) (OtherBodyIndex :type Integer) (bFromSweep :type Boolean) (SweepResult :type Hit%20Result%20Structure%20%28by%20ref%29))
  ;[1 1 1] Overlap - Set HeroOnSight
  (Variables|Default|SetisHeroOnSight true))

(event Custom|StopEnemy
  ;[1 1 1] Inimigo Para
  (Utilities|Time|ClearTimerbyFunctionName 0 "Fire"))

(event Custom|RestartEnemyFire
  ;[1 1 1] Set Actor Rotation - Olha para o Jogador
  (Utilities|FlowControl|DoOnce false) ; enters at Reset
)

(event Custom|EnemyDead)

(event Custom|RestartEnemy
  ;[1 1 1] Inimigo Reinicia
  (Variables|Default|SetisHeroOnSight false)
  (Variables|Default|SetisHeroHere false))

(event EventBeginPlay
  (bind _returnvalue (Transformation|GetActorLocation))
  (Utilities|FlowControl|Sequence
    (:then_0
      ;[1 1 1] Set Start End Location / Set Timeline Play Rate
      (Variables|Default|SetStartLocation _returnvalue)
      (Variables|Default|SetEndLocation (+ _returnvalue (Math|Vector|MakeVector 0.0 0.0 (Math|Random|RandomFloatinRange 5e+01 1e+02))))
      (Components|Timeline|SetPlayRate (Variables|Default|GetEnemyLoop) (Math|Random|RandomFloatinRange 1.0 2.0)))
    (:then_1
      ;[1 1 1] Get Hero Char Refer
      (bind _asbp_hero_char (Utilities|Casting|CastToBP_HeroChar (Game|GetPlayerCharacter 0)))
      (Variables|Default|SetHeroCharRefer _asbp_hero_char))))

(event EventTick
  (params (DeltaSeconds :type Float%20%28single-precision%29))
  ;[1 1 1] Set Actor Rotation - Olha para o Jogador
  (if (or (Variables|Default|GetisHeroOnSight) (Variables|Default|GetisHeroHere))
    (Utilities|FlowControl|Sequence
      (:then_0
        (Transformation|SetActorRotation (Math|Rotator|FindLookatRotation (Transformation|GetActorLocation) (Transformation|GetActorLocation (Variables|Default|GetHeroCharRefer)))))
      (:then_1
        (Utilities|FlowControl|DoOnce false
          (:Completed
            (Utilities|Time|SetTimerbyFunctionName 0 "Fire" (/ 1.0 (Variables|Default|GetShootPerSecond)) true)))))))

(event Collision|EventHit
  (params (MyComp :type Primitive%20Component%20Object%20Reference) (Other :type Actor%20Object%20Reference) (OtherComp :type Primitive%20Component%20Object%20Reference) (bSelfMoved :type Boolean) (HitLocation :type Vector :default "0, 0, 0") (HitNormal :type Vector :default "0, 0, 0") (NormalImpulse :type Vector :default "0, 0, 0") (Hit :type Hit%20Result%20Structure%20%28by%20ref%29))
  ;[1 1 1] Hit
  ;;[0.401 0.345 0.01253] Play Sound
  (Audio|PlaySoundatLocation "/Game/Audio/grenade2_Cue.grenade2_Cue" HitLocation "0, 0, 0" 1.0 1.0 0.0 0 0 0)
  (Variables|Default|SetisHeroHere true)
  (Variables|Default|SetEnemyHealth (- (Variables|Default|GetEnemyHealth) (Variables|Default|GetDamageTaken)))
  (if (<= (Variables|Default|GetEnemyHealth) 0.0)
    (CallFunction|EnemyDead)
    (Actor|DestroyActor)
    (else
      (Rendering|Material|SetScalarParameterValueonMaterials (Variables|Default|GetEnemyMesh) "Emissive" 1.0)
      (Utilities|FlowControl|Delay 0.1)
      (Rendering|Material|SetScalarParameterValueonMaterials (Variables|Default|GetEnemyMesh) "Emissive" 6e+01))))

(fn ConstructionScript)

(fn Fire
  (bind _arrowprojetil (Variables|Default|GetArrowProjetil))
  (bind _arrowprojetil_2 (Variables|Default|GetArrowProjetil))
  (Game|SpawnActorfromClass "/Game/Enemy/BP_ProjetilEnemy.BP_ProjetilEnemy_C" (Transformation|GetWorldTransform _arrowprojetil) "Undefined" 0 0)
  (if (Variables|Default|GetbIsBoss)
    (Game|SpawnActorfromClass "/Game/Enemy/BP_ProjetilEnemy.BP_ProjetilEnemy_C" (Transformation|GetWorldTransform _arrowprojetil_2) "Undefined" 0 0)
    (Audio|PlaySoundatLocation "/Game/Audio/tiro6_CueBoss.tiro6_CueBoss" (Transformation|GetWorldLocation _arrowprojetil_2) "0, 0, 0" 1.0 1.0 0.0 0 0 0)
    (else
      ;[0.2344 0.1817 0.004883] Toca Audio de Projetil
      (Audio|PlaySoundatLocation "/Game/Audio/tiro6_Cue.tiro6_Cue" (Transformation|GetWorldLocation _arrowprojetil) "0, 0, 0" 1.0 1.0 0.0 0 0 0))))